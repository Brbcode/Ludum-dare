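; Player controller for a game that alternates between main-character control and a minions' turn, with camera blends before possessing either.
; On BeginPlay it maps owned minions to slots using the last digit of their names.
; Movement is blocked during the minions' turn, when a press and release on the same owned minion records an action.
; Once every minion has one, it notifies the game mode, which also handles mode changes.
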(event `self.ReceiveBeginPlay`
  ;[1 1 1] Set internal game mode variable
  (bind _asbp_game_mode (cast `/Game/GameModes/bp_GameMode` (`GameplayStatics.GetGameMode`)))
  (set `self.GameMode` _asbp_game_mode)
  ;[1 1 1] Set internal controller id variable
  (bind _returnvalue (`GameplayStatics.GetPlayerControllerID` self))
  (set `self.ControllerId` _returnvalue)
  ;[1 1 1] Initialize main character
  (bind _asbp_player (cast `/Game/Blueprints/bpPlayer` (`self.K2_GetPawn`)))
  (set `self.MainCharacter` _asbp_player)
  ;[1 1 1] Get owning minions
  (bind _outactors (`GameplayStatics.GetAllActorsOfClass` "/Game/Blueprints/bpMinion.bpMinion_C"))
  (for _array_element _outactors
    (if (== (`self.ControllerId`) (`/Game/Blueprints/bpMinion.PlayerOwner` _array_element))
      (bind _returnvalue_2 (`KismetSystemLibrary.GetDisplayName` _array_element))
      (`BlueprintMapLibrary.Map_Add` (`self.PositionToMinions`) (- (`KismetStringLibrary.Conv_StringToInt` (`KismetStringLibrary.GetSubstring` _returnvalue_2 (- (`KismetStringLibrary.Len` _returnvalue_2) 1))) 1) _array_element))))

(event `InputAction|ChangeMode`
  (params (Key :type "Key Structure"))
  ;[1 1 1] Change Mode
  (:`Pressed`
    (`/Game/GameModes/bp_GameMode.ChangeMode` (`self.GameMode`))))

(event `InputAction|ChangeToPosition`
  (params (Key :type "Key Structure"))
  (bind _camerachangedelay (`self.CameraChangeDelay`))
  (bind _value (`BlueprintMapLibrary.Map_Find` (`self.PositionToMinions`) (`BlueprintMapLibrary.Map_Find` (`self.KeyToNumber`) Key)))
  ;[1 1 1] Change possesed pawn
  (:`Pressed`
    (`self.SetViewTargetWithBlend` _value _camerachangedelay)
    (`KismetSystemLibrary.Delay` _camerachangedelay)
    (`self.Possess` _value)))

(event `InputAction|ChangeToMainCharacter`
  (params (Key :type "Key Structure"))
  (bind _maincharacter (`self.MainCharacter`))
  (bind _camerachangedelay (`self.CameraChangeDelay`))
  ;[1 1 1] Change possesed pawn
  (:`Pressed`
    (`self.SetViewTargetWithBlend` _maincharacter _camerachangedelay)
    (`KismetSystemLibrary.Delay` _camerachangedelay)
    (`self.Possess` _maincharacter)))

(event `InputAxis|Vertical`
  (params (AxisValue :type "Float (single-precision)"))
  ;[1 1 1] Movement
  (bind _isminionsturn (`self.IsMinionsTurn`))
  (if (not _isminionsturn)
    (`/Game/Blueprints/bpPlayer.Move` (`self.MainCharacter`) (`KismetMathLibrary.MakeVector` AxisValue (stale `InputAxis|Horizontal` AxisValue)) 10.0 :!label _label)))

(event `InputAxis|Horizontal`
  (params (AxisValue :type "Float (single-precision)"))
  ;[1 1 1] Movement
  (goto _label))

(event `InputAction|Attack`
  (params (Key :type "Key Structure"))
  ;[1 1 1] Attack
  (:`Pressed`
    (`/Game/Blueprints/bpPlayer.Attack` (`self.MainCharacter`))))

(event `onMinionActionChosen`
  ;[1 1 1] On minion action chosen
  ;;[1 1 1] Check if it is minions turn
  (bind _isminionsturn (`self.IsMinionsTurn`))
  (if _isminionsturn
    ;;[1 1 1] Check number of minion actions taken
    (if (== (`BlueprintMapLibrary.Map_Length` (`self.ActionsChoosen`)) (`BlueprintMapLibrary.Map_Length` (`self.PositionToMinions`)))
      ;;[1 1 1] Notify game mode that every minion has chosen its actions
      (`/Game/GameModes/bp_GameMode.onMinionActionChosen` (`self.GameMode`) (`self.ControllerId`)))))

(event `InputAction|ChooseFirstAction`
  (params (Key :type "Key Structure"))
  ;[1 1 1] Add attack action to the pile
  (:`Pressed`
    (`self.GetReleaseClickMinion` true))
  (:`Released`
    (bind (_minion _exists) (`self.GetReleaseClickMinion` false))
    (if _exists
      (`KismetSystemLibrary.PrintString` "Chosen action 1")
      (`BlueprintMapLibrary.Map_Add` (`self.ActionsChoosen`) _minion)
      (`self.onMinionActionChosen`))))

(event `InputAction|ChooseSecondAction`
  (params (Key :type "Key Structure"))
  ;[1 1 1] Add second action to the pile
  (:`Pressed`
    (`self.GetReleaseClickMinion` true))
  (:`Released`
    (bind (_minion _exists) (`self.GetReleaseClickMinion` false))
    (if _exists
      (`KismetSystemLibrary.PrintString` "Chosen action 2")
      (`BlueprintMapLibrary.Map_Add` (`self.ActionsChoosen`) _minion "NewEnumerator1")
      (`self.onMinionActionChosen`))))

(fn `GetClickedOwnedMinion`
  (returns (Minion :type "/Game/Blueprints/bpMinion Object Reference") (MinionClicked :type Boolean))
  (bind _isminionsturn (`self.IsMinionsTurn`))
  (if _isminionsturn
    (bind _asbp_minion (cast `/Game/Blueprints/bpMinion` (`.HitActor` (`GameplayStatics.BreakHitResult` (`self.GetHitResultUnderCursorForObjects` (`|MakeArray` "ObjectTypeQuery3" :!type "EObjectTypeQuery Enum"))))))
    (bind _values (`BlueprintMapLibrary.Map_Values` (`self.PositionToMinions`)))
    (if (`KismetArrayLibrary.Array_Contains` _values _asbp_minion)
      (return _asbp_minion true)
      (else
        _)))
  (return null false))

(fn `GetReleaseClickMinion`
  (params (IsEnterEvent :type Boolean :default true))
  (returns (Minion :type "/Game/Blueprints/bpMinion Object Reference") (Exists :type Boolean))
  (if IsEnterEvent
    (bind (_minion _minionclicked) (`self.GetClickedOwnedMinion`))
    (if _minionclicked
      (set `self.PressedMinion` _minion))
    (else
      (bind (_minion_2 _minionclicked_2) (`self.GetClickedOwnedMinion`))
      (return _minion_2 (and _minionclicked_2 (== _minion_2 (`self.PressedMinion`)))))))

(fn `IsMinionsTurn`
  (returns (IsMinionsTurn :type Boolean))
  (return (`/Game/GameModes/bp_GameMode.IsMinionTurn` (`self.GameMode`))))

(fn `UserConstructionScript`)