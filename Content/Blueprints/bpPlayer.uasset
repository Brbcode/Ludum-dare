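; Player pawn for a game that alternates player and minion turns, with health, attack, move and steal actions.
; Each action runs only when IsPlayerTurn finds bp_GameMode's IsMinionTurn false; Move then applies movement input.
; Attack and Steal only print messages so far, though Attack has a delay-based cooldown.
; Tick prints an elimination message with the controller ID every frame while health is depleted.
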(event `self.ReceiveBeginPlay`
  ;[1 1 1] Initialization
  (set `self.Health` (`self.MaxHealth`))
  (set `self.CanAttack` true)
  (set `self.CanMove` false))

(event `self.ReceiveTick`
  (params (DeltaSeconds :type "Float (single-precision)"))
  ;[1 1 1] Check player health
  (if (<= (`self.Health`) 0)
    (bind _returnvalue (`GameplayStatics.GetPlayerControllerID` null))
    (`KismetSystemLibrary.PrintString` (`KismetStringLibrary.Concat_StrStr` "Jugador " (`KismetStringLibrary.Conv_IntToString` _returnvalue) " eliminado"))))

(event `Attack`
  ;[1 1 1] Attack event
  (bind _isplayerturn (`self.IsPlayerTurn`))
  (if (and _isplayerturn (`self.CanAttack`))
    (set `self.CanAttack` false)
    (bind _returnvalue (`GameplayStatics.GetPlayerControllerID` null))
    (`KismetSystemLibrary.PrintString` (`KismetStringLibrary.Concat_StrStr` "Jugador " (`KismetStringLibrary.Conv_IntToString` _returnvalue) " ataca"))
    (`KismetSystemLibrary.Delay` (`self.AttackDelay`))
    (set `self.CanAttack` true)))

(event `Move`
  (params (Direction :type "Vector Structure") (Scale :type "Float (double-precision)"))
  ;[1 1 1] Move event
  (bind _isplayerturn (`self.IsPlayerTurn`))
  (if _isplayerturn
    (`self.AddMovementInput` Direction Scale)))

(event `Steal`
  ;[1 1 1] Steal
  (bind _isplayerturn (`self.IsPlayerTurn`))
  (if _isplayerturn
    (`KismetSystemLibrary.PrintString` "Steal")))

(fn `IsPlayerTurn`
  (returns (IsPlayerTurn :type Boolean))
  (bind _asbp_game_mode (cast `/Game/GameModes/bp_GameMode` (`GameplayStatics.GetGameMode`)))
  (return (not (`/Game/GameModes/bp_GameMode.IsMinionTurn` _asbp_game_mode))))

(fn `UserConstructionScript`)