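; Minion Blueprint for a turn-based combat game, holding stats, an element type and an attack action.
; On BeginPlay it fills health to maximum, rolls attack, defense and velocity randomly, picks a random element and flags itself able to act.
; The attack event asks bp_GameMode whether it is the minions' turn, then only prints a debug message with the player controller ID and briefly delays; no damage is applied.
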(event `self.ReceiveBeginPlay`
  (`self.Initialize`))

(event `Initialize`
  ;[1 1 1] Initialization
  (set `self.Health` (`self.MaxHealth`))
  (set `self.Attack` (`KismetMathLibrary.RandomIntegerInRange` 50 100))
  (set `self.Defense` (`KismetMathLibrary.RandomIntegerInRange` 50 100))
  (set `self.Velocity` (`KismetMathLibrary.RandomIntegerInRange` 50 100))
  (set `self.ElementType` (cast `/Game/GameModes/EnumElementTypes` (`KismetMathLibrary.Conv_IntToByte` (`KismetMathLibrary.RandomIntegerInRange` 0 (- (enumcount `/Game/GameModes/EnumElementTypes`) 1)))))
  (set `self.canActuate` true))

(event `CustomEvent`
  ;[1 1 1] Attack event
  (bind _isminionsturn (`self.IsMinionsTurn`))
  (if _isminionsturn
    (bind _returnvalue (`GameplayStatics.GetPlayerControllerID` null))
    (`KismetSystemLibrary.PrintString` (`KismetStringLibrary.Concat_StrStr` "Minion " (`KismetStringLibrary.Conv_IntToString` _returnvalue) " ataca"))
    (`KismetSystemLibrary.Delay` 0.2)))

(fn `IsMinionsTurn`
  (returns (IsMinionsTurn :type Boolean))
  (bind _asbp_game_mode (cast `/Game/GameModes/bp_GameMode` (`GameplayStatics.GetGameMode`)))
  (return (`/Game/GameModes/bp_GameMode.IsMinionTurn` _asbp_game_mode)))

(fn `UserConstructionScript`)