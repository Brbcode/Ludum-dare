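; Game mode for a two-player game with minion turns, tracking when both players have chosen their minion actions.
; On begin play it creates a player on controller 0 and shows that player's mouse cursor.
; Each action-chosen event flags its player, and once both flags are set it calls RunMinionsActions, which only prints a message.
; ChangeMode toggles the minion-turn flag and fires OnChangeMode, also a print stub.
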(event `self.ReceiveBeginPlay`
  (`GameplayStatics.CreatePlayer` 0)
  (set `PlayerController.bShowMouseCursor` true (`GameplayStatics.GetPlayerController` 0)))

(event `onMinionActionChosen`
  (params (PlayerControllerId :type Integer))
  ;[1 1 1] Check minion actions chosen
  (if (== PlayerControllerId 0)
    (bind _output_get (set `self.Player1MinionsActionsChosen` true))
    (`KismetSystemLibrary.PrintString` "Player 1 minion actons chosen")
    (else
      (bind _output_get_2 (set `self.Player2MinionsActionsChosen` true))))
  (if (and _output_get _output_get_2)
    (`self.RunMinionsActions`)))

(event `RunMinionsActions`
  (`KismetSystemLibrary.PrintString` "All actions chosen"))

(event `ChangeMode`
  (set `self.IsMinionTurn` (not (`self.IsMinionTurn`)))
  (`self.OnChangeMode`))

(event `OnChangeMode`
  (`KismetSystemLibrary.PrintString` "Mode Changed"))

(fn `UserConstructionScript`)